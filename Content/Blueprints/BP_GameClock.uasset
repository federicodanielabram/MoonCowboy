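; Game clock actor that turns time since its creation into an accelerated day and time readout and rotates a sun light.
; Each Tick, chained MapRangeUnclamped nodes act as unit converters, with modulo and fraction splitting out hours, minutes and seconds.
; The same elapsed time drives the SunLight's yaw at fixed pitch.
; The Spanish-formatted DisplayText is also printed every frame, and UpdateDisplay copies it to a given text target.
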(event `self.ReceiveTick`
  (params (DeltaSeconds :type "Float (single-precision)"))
  (bind _returnvalue (`KismetMathLibrary.MapRangeUnclamped` (`self.GetGameTimeSinceCreation` self) 0.0 60.0 0.0 1.0))
  (bind _returnvalue_2 (`KismetMathLibrary.MapRangeUnclamped` _returnvalue 0.0 2.0 0.0 1.0))
  (bind _returnvalue_3 (mod _returnvalue_2 24.0))
  (bind _returnvalue_4 (`KismetMathLibrary.MapRangeUnclamped` (`KismetMathLibrary.Fraction` _returnvalue_3) 0.0 1.0 0.0 60.0))
  (bind _result (`|FormatText` "Día {Day} - {HH}:{MM}:{SS}" (`KismetMathLibrary.FFloor` (`KismetMathLibrary.MapRangeUnclamped` _returnvalue_2 0.0 24.0 0.0 1.0)) (`KismetMathLibrary.FFloor` _returnvalue_3) (`KismetMathLibrary.FFloor` _returnvalue_4) (`KismetMathLibrary.FFloor` (`KismetMathLibrary.MapRangeUnclamped` (`KismetMathLibrary.Fraction` _returnvalue_4) 0.0 1.0 0.0 60.0))))
  (set `self.T` _returnvalue)
  (`self.K2_SetActorRotation` (`self.SunLight`) (`KismetMathLibrary.MakeRotator` 0.0 -1.54 (`KismetMathLibrary.MapRangeUnclamped` (`KismetMathLibrary.MapRangeUnclamped` _returnvalue 0.0 1.0 255.1 254.846) 0.0 1.0 180.0 181.0)) false)
  (set `self.DisplayText` _result)
  (`KismetSystemLibrary.PrintString` (`KismetTextLibrary.Conv_TextToString` _result) true false (struct :`G` 0.66 :`B` 1.0 :`A` 1.0) 0.1 "ClockDisplay"))

(fn `UpdateDisplay`
  (params (Target :type "TextBlock Object Reference"))
  (`TextBlock.SetText` Target (`self.DisplayText`)))

(fn `UserConstructionScript`)